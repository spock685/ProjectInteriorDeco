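; BP_DamageNumberActor is a short-lived actor that displays a floating damage number.
; On BeginPlay it passes its Damage value to the W_FloatingDamage widget in its widget component and launches its static mesh with a random upward, sideways-scattered velocity impulse.
; It destroys itself when the widget reports that its lifetime is over, with a fixed delay as fallback.
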(event `self.ReceiveBeginPlay`
  (`|ExecutionSequence`
    (:`then_0`
      (`KismetSystemLibrary.Delay` 3.0)
      (`/Engine/EditorBlueprintResources/StandardMacros.IsValid` self
        (:`Is Valid`
          (`self.K2_DestroyActor` :!label _label))))
    (:`then_1`
      (bind _asw_floating_damage (cast `/Game/NewAssets/FloatingDamageNumbers/W_FloatingDamage` (`WidgetComponent.GetUserWidgetObject` (`self.Widget`))))
      (add `/Game/NewAssets/FloatingDamageNumbers/W_FloatingDamage.WidgetLifetimeOver` _asw_floating_damage (delegate `WidgetDead`))
      (message `/Game/NewAssets/FloatingDamageNumbers/BPI_SetDamageValue.SetDamageValue` _asw_floating_damage (`self.Damage`))
      (`PrimitiveComponent.AddImpulse` (`self.StaticMesh`) (`KismetMathLibrary.MakeVector` (`KismetMathLibrary.RandomFloatInRange` -400.0 400.0) (`KismetMathLibrary.RandomFloatInRange` -400.0 400.0) (`KismetMathLibrary.RandomFloatInRange` 400.0 800.0)) "None" true))))

(event `WidgetDead`
  (goto _label))

(fn `UserConstructionScript`)